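; Game Instance Blueprint that holds player HP in the GameST struct and handles losing the game.
; DecreaseHP rebuilds the struct with less HP; when HP runs out, it shows the WBP_LostScrean widget and returns to the main menu level after a short delay.
; Init calls CallED1 following a zero-length delay.
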(event `DecreaseHP`
  (bind _game_st_hp (break `/Game/GameInstance/BP_MyGameStructure` (`self.Game ST`)))
  (bind _output_get (set `self.Game ST` (make `/Game/GameInstance/BP_MyGameStructure` (- _game_st_hp 10))))
  (if (<= (`.HP_2_13F61D32436C3FD89116648CD567BFB2` (break `/Game/GameInstance/BP_MyGameStructure` _output_get)) 0)
    (bind _returnvalue (`|CreateWidget` "/Game/GameWidgets/MessageScrean/WBP_LostScrean.WBP_LostScrean_C"))
    (`UserWidget.AddToViewport` _returnvalue 0)
    (`KismetSystemLibrary.Delay` 2.0)
    (`GameplayStatics.OpenLevel` "MainMenu_lvl")))

(event `self.ReceiveInit`
  (`KismetSystemLibrary.Delay` 0.0)
  (`self.ED1`))