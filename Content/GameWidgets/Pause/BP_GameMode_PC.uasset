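; BP_GameMode_PC is a player controller that toggles the pause menu on the Pause input action.
; Pausing freezes the game, shows the cursor, creates WBP_Pause, switches input to game and UI, and plays the widget's animation.
; Unpausing resumes the game and hides the cursor, plays the reverse animation, then after a short delay removes the widget and restores game-only input.
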(event `InputAction|Pause` :paused true
  (params (Key :type "Key Structure"))
  (bind _returnvalue (`GameplayStatics.GetPlayerController` 0))
  (:`Pressed`
    (if (`GameplayStatics.IsGamePaused`)
      (`GameplayStatics.SetGamePaused` false)
      (set `self.bShowMouseCursor` false)
      (`/Game/GameWidgets/Pause/WBP_Pause.RevercePlayAnim` (stale _returnvalue_2))
      (`KismetSystemLibrary.Delay` 1.0)
      (`Widget.RemoveFromParent` (stale _returnvalue_2))
      (`WidgetBlueprintLibrary.SetInputMode_GameOnly` _returnvalue)
      (else
        (`GameplayStatics.SetGamePaused` true)
        (set `self.bShowMouseCursor` true)
        (bind _returnvalue_2 (`|CreateWidget` "/Game/GameWidgets/Pause/WBP_Pause.WBP_Pause_C"))
        (`UserWidget.AddToViewport` _returnvalue_2 0)
        (`WidgetBlueprintLibrary.SetInputMode_GameAndUIEx` _returnvalue _returnvalue_2)
        (`/Game/GameWidgets/Pause/WBP_Pause.PlayAnim` _returnvalue_2)))))

(fn `UserConstructionScript`)